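; Jump-scare picture frame that gets knocked loose when something overlaps its trigger box.
; If overlap triggering is enabled, the first overlap waits a delay, then unhides the frame and turns on physics and collision.
; It then applies an impulse at world origin, adding the strength to the forward vector rather than scaling it.
; The construction script scales the trigger from OverlapBox and offsets it along negative Y to match.
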(event OnComponentBeginOverlap(Box)
  (params (OverlappedComponent :type Primitive%20Component%20Object%20Reference) (OtherActor :type Actor%20Object%20Reference) (OtherComp :type Primitive%20Component%20Object%20Reference) (OtherBodyIndex :type Integer) (bFromSweep :type Boolean) (SweepResult :type Hit%20Result%20Structure%20%28by%20ref%29))
  (bind _pictureframe (Variables|Default|GetPictureFrame))
  ;[1 1 1] Use the Overlap
  (if (Variables|Default|GetUseOverlaping)
    (Utilities|FlowControl|DoOnce false
      (:Completed
        (Utilities|FlowControl|Delay (Variables|Default|GetImpulseDelay))
        ;;[1 1 1] Enable Physic
        (Physics|SetSimulatePhysics _pictureframe true)
        (Collision|SetCollisionEnabled _pictureframe "QueryAndPhysics")
        (Development|SetHiddeninGame _pictureframe false false)
        (Physics|AddImpulseatLocation (Variables|Default|GetPictureFrame) (+ (Math|Vector|GetForwardVector (Variables|Default|GetPictureFrame)) (Variables|Default|GetImpulseStrength)) "0, 0, 0" "None")))))

(fn ConstructionScript
  ;[1 1 1] Change the Overlapbox
  (Transformation|SetRelativeTransform (Variables|Default|GetBox) (Math|Transform|MakeTransform (Math|Vector|MakeVector 0.0 (- 0.0 (* (.y (Variables|Default|GetOverlapBox)) 1e+01)) 0.0) "0, 0, 0" (Variables|Default|GetOverlapBox)) false false))