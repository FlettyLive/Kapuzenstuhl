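; Vision helper whose IsInViewport function tests whether an actor is horizontally within player 0's screen.
; It projects the bounds origin and an X-extent offset to screen space, using their distance as an on-screen radius.
; The origin's screen X must lie between minus that radius and twice the viewport width less radius; Y and Tolerance are unused.
; Debug prints and a debug line from deprojected position to direction remain.
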(fn IsinViewport
  (params (object :type Actor%20Object%20Reference) (tolerance :type Integer))
  (bind (_origin _boxextent) (Collision|GetActorBounds object false))
  (bind _returnvalue (Game|GetPlayerController 0))
  (bind _returnvalue_2 (Viewport|GetViewportSize))
  (bind _screenlocation (Class|PlayerController|ProjectWorldLocationtoScreen _returnvalue _origin))
  (bind _x (Math|Vector|BreakVector _boxextent))
  (bind _returnvalue_3 (Math|Vector|MakeVector _x 0.0 0.0))
  (bind _x_2 (Math|Vector2D|BreakVector2D _screenlocation))
  (bind _returnvalue_4 (+ _origin _returnvalue_3))
  (bind _screenlocation_2 (Class|PlayerController|ProjectWorldLocationtoScreen _returnvalue _returnvalue_4))
  (bind _returnvalue_5 (- _screenlocation _screenlocation_2))
  (bind (_worldposition _worlddirection) (Class|GameplayStatics|DeprojectScreentoWorld _returnvalue _screenlocation_2))
  (bind _returnvalue_6 (Math|Vector2D|Vector2DLength _returnvalue_5))
  (Development|PrintString 0 (Utilities|String|ToString(Float) (.x _returnvalue_2)))
  (Development|PrintString 0 (Utilities|String|ToString(Float) _returnvalue_6))
  (Rendering|Debug|DrawDebugLine 0 _worldposition _worlddirection "(R=0.595000,G=0.000000,B=0.044042,A=1.000000)" 0.0 0.0)
  (return (and (> (* (- (.x _returnvalue_2) _returnvalue_6) 2.0) _x_2) (> _x_2 (* -1 _returnvalue_6)))))