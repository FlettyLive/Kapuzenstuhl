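; Blueprint helper functions that start a yes/no prompt through the player controller and read back its answer.
; CallYesNo prints "Yes or No?" and calls StartYesNo on player 0's PlayerCon.
; CallYesNoResult separately returns that controller's YesNoAnswer, so starting the prompt and fetching the result are two independent calls.
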(fn CallYesNo
  (Development|PrintString 0 "Yes or No?")
  (bind _asplayer_con (Utilities|Casting|CastToPlayerCon (Game|GetPlayerController 0)))
  (bind _output_get (LocalVariables|SetPlayerCon _asplayer_con))
  (Default|StartYesNo _output_get))

(fn CallYesNoResult
  (bind _asplayer_con (Utilities|Casting|CastToPlayerCon (Game|GetPlayerController 0)))
  (bind _output_get (LocalVariables|SetPlayerCon _asplayer_con))
  (return (Variables|/Game/Blueprints/System/PlayerCon.PlayerCon_C|GetYesNoAnswer _output_get)))