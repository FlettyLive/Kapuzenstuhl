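; PlaySound is a helper function that spawns a sound at the world location of a given component, without attaching it, and returns the audio component.
; A valid CustomAttenuation asset is applied at spawn, followed by a fade-in using the supplied duration and volume.
; Otherwise UseAttenuation is applied after spawning through AdjustAttenuation.
; That fallback branch ignores the fade inputs and calls FadeIn with zero duration and zero volume.
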(fn PlaySound
  (params (Sound :type Sound%20Base%20Object%20Reference) (Attached :type Scene%20Component%20Object%20Reference) (Use%20Attenuation :type Attenuation%20Settings%20Structure) (Custom%20Attenuation :type Sound%20Attenuation%20Object%20Reference) (Fade%20Duration :type Float%20%28single-precision%29) (Fade%20Volume%20Level :type Float%20%28single-precision%29))
  (if (Utilities|IsValid Custom%20Attenuation)
    ;[1 1 1] User Attenuation Setting
    (bind _returnvalue (Audio|SpawnSoundatLocation 0 Sound (Transformation|GetWorldLocation Attached) "0, 0, 0" 1.0 1.0 0.0 Custom%20Attenuation))
    (bind _output_get (LocalVariables|SetAudioComp _returnvalue))
    (Audio|Components|Audio|FadeIn _output_get Fade%20Duration Fade%20Volume%20Level 0.0 :!class /Script/Engine.AudioComponent)
    (return _output_get)
    (else
      ;[1 1 1] Use Custom Attenuation Setting
      (bind _returnvalue_2 (Audio|SpawnSoundatLocation 0 Sound (Transformation|GetWorldLocation Attached)))
      (bind _output_get_2 (LocalVariables|SetAudioComp _returnvalue_2))
      (Utilities|FlowControl|Sequence
        (:then_0
          (Audio|Components|Audio|FadeIn _output_get_2 0.0 0.0 0.0 :!class /Script/Engine.AudioComponent))
        (:then_1
          (Audio|Components|Audio|AdjustAttenuation _output_get_2 Use%20Attenuation)
          (return _output_get_2))))))