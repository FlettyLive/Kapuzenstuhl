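; Blueprint function library with a helper, GetColBox, that returns a random world point within a box collision component.
; It adds a random offset on each axis, bounded by the scaled box extent in both directions, to the component's world location.
; The offset ignores the component's rotation, so sampled points follow world axes even when the box is rotated.
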(fn GetColBox
  (params (BoxCollision :type Box%20Component%20Object%20Reference))
  (bind _returnvalue (Components|Box|GetScaledBoxExtent BoxCollision))
  (bind (_x _y _z) (Math|Vector|BreakVector _returnvalue))
  (return (+ (Transformation|GetWorldLocation BoxCollision) (Math|Vector|MakeVector (Math|Random|RandomFloatinRange (* _x -1.0) _x) (Math|Random|RandomFloatinRange (* _y -1.0) _y) (Math|Random|RandomFloatinRange (* _z -1.0) _z)))))