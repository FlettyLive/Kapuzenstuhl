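; Horror picture frame prop that is knocked loose when something overlaps its trigger box, if overlap triggering is enabled.
; A one-shot overlap waits a delay, then enables physics and collision, unhides the frame and applies an impulse along the Arrow component.
; Hits above an impulse threshold play an attenuated falling sound.
; The construction script places the box and arrow from variables, mapping a 2D point to the arrow's X and Z.
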(event OnComponentBeginOverlap(Box)
  (params (OverlappedComponent :type Primitive%20Component%20Object%20Reference) (OtherActor :type Actor%20Object%20Reference) (OtherComp :type Primitive%20Component%20Object%20Reference) (OtherBodyIndex :type Integer) (bFromSweep :type Boolean) (SweepResult :type Hit%20Result%20Structure%20%28by%20ref%29))
  (bind _arrow (Variables|Default|GetArrow))
  (bind _pictureframe (Variables|Default|GetPictureFrame))
  ;[1 1 1] Use the Overlap
  (if (Variables|Default|GetUseOverlaping)
    (Utilities|FlowControl|DoOnce false
      (:Completed
        (Utilities|FlowControl|Delay (Variables|Default|GetImpulseDelay))
        ;;[1 1 1] Enable Physic
        (Physics|SetSimulatePhysics _pictureframe true)
        (Collision|SetCollisionEnabled _pictureframe "QueryAndPhysics")
        (Development|SetHiddeninGame _pictureframe false false)
        (Physics|AddImpulseatLocation _pictureframe (* (Math|Vector|GetForwardVector _arrow) (Variables|Default|GetImpulseStrength)) (Transformation|GetWorldLocation _arrow) "None")))))

(event OnComponentHit(PictureFrame)
  (params (HitComponent :type Primitive%20Component%20Object%20Reference) (OtherActor :type Actor%20Object%20Reference) (OtherComp :type Primitive%20Component%20Object%20Reference) (NormalImpulse :type Vector) (Hit :type Hit%20Result%20Structure%20%28by%20ref%29))
  ;[1 1 1] Falling Sound
  (if (> (Math|Vector|VectorLength NormalImpulse) (Variables|Default|GetFalling%20Sound%20Impulse))
    (Audio|PlaySoundatLocation (Variables|Default|GetFalling%20Sound) (Transformation|GetWorldLocation (Variables|Default|GetPictureFrame)) "0, 0, 0" 1.0 1.0 0.0 (Variables|Default|GetSound%20Attenuation))))

(fn ConstructionScript
  (bind _arrowposition__impulsepoint_ (Variables|Default|GetArrowPosition%20%28Impulsepoint%29))
  ;[1 1 1] Change the Overlapbox
  (Utilities|FlowControl|Sequence
    (:then_0
      (Transformation|SetRelativeTransform (Variables|Default|GetBox) (Math|Transform|MakeTransform (Variables|Default|GetOverlapBoxPosition) (Variables|Default|GetOverlapBoxRotation) (Variables|Default|GetOverlapBoxScale)) false false))
    (:then_1
      ;[1 1 1] Change the Arrow
      (Transformation|SetRelativeLocation (Variables|Default|GetArrow) (Math|Vector|MakeVector (.x _arrowposition__impulsepoint_) 0.0 (.y _arrowposition__impulsepoint_)) false false))))