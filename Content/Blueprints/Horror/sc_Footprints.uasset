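; Horror effect actor that lays a trail of alternating left and right footprints along an arrow's forward direction, on BeginPlay if StartInstant is set.
; StartFootprint re-calls itself after a delay until the step count is reached, offsetting each print by the truncated count times distance.
; Each step plays a sound at world origin, then a FlipFlop picks the foot for the optional yaw-aligned, timed decal and optional particle effect.
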(event Custom|StartFootprint
  (bind _footprint_angle_l (Variables|Default|GetFootprint%20Angle%20L))
  (bind _footprint_angle_r (Variables|Default|GetFootprint%20Angle%20R))
  (bind _footprint_size (Variables|Default|GetFootprint%20Size))
  (bind _arrow (Variables|Default|GetArrow))
  (bind _footprint_size_2 (Variables|Default|GetFootprint%20Size))
  (bind _returnvalue (Transformation|GetWorldRotation _arrow))
  (bind _yaw (Math|Rotator|BreakRotator _returnvalue))
  (bind _yaw_2 (Math|Rotator|BreakRotator _returnvalue))
  (bind _returnvalue_2 (+ _yaw _footprint_angle_r))
  (bind _returnvalue_3 (+ _yaw_2 _footprint_angle_l))
  (bind _returnvalue_4 (Math|Rotator|MakeRotator _returnvalue_2 -9e+01 0.0))
  (bind _returnvalue_5 (Math|Rotator|MakeRotator _returnvalue_3 -9e+01 0.0))
  ;[1 1 1] Add Footprints step by step
  (Utilities|FlowControl|Delay (Variables|Default|GetFootprint%20Delay))
  (Audio|PlaySoundatLocation (Variables|Default|GetFootstep%20Sound) "0, 0, 0" "0, 0, 0" 1.0 1.0 0.0 (Variables|Default|GetSound%20Attenuation))
  (Variables|Default|SetFootprint%20Location (+ (Transformation|GetWorldLocation _arrow) (* (Math|Vector|GetForwardVector _returnvalue) (Math|Conversions|ToFloat(Integer) (Math|Float|Truncate (* (Variables|Default|GetFootprint%20Count%20Cur) (Variables|Default|GetFootprint%20Distance)))))))
  (Utilities|FlowControl|FlipFlop
    (:A
      (Utilities|FlowControl|Sequence
        (:then_0
          ;;[1 1 1] Decal and Effect
          (if (Variables|Default|GetDecalsOn)
            (Rendering|Decal|SpawnDecalatLocation (Variables|Default|GetFoot_L) (Math|Vector|MakeVector 1.0 _footprint_size_2 _footprint_size_2) (Variables|Default|GetFootprint%20Location) _returnvalue_5 (Variables|Default|GetFootprint%20Lifetime))))
        (:then_1
          (if (Variables|Default|GetEffectOn)
            (Effects|SpawnEmitteratLocation "/Game/InfinityBladeEffects/Effects/FX_Combat_Base/Notifies/P_FootSteps_Walk.P_FootSteps_Walk" (Variables|Default|GetFootprint%20Location) _returnvalue_5)))
        (:then_2
          ;[1 1 1] Calc to next Step
          (Variables|Default|SetFootprint%20Count%20Cur (+ (Variables|Default|GetFootprint%20Count%20Cur) 1) :!label _label)
          (if (!= (Variables|Default|GetFootprint%20Count%20Cur) (Variables|Default|GetFootprint%20Count))
            (CallFunction|StartFootprint)))))
    (:B
      (Utilities|FlowControl|Sequence
        (:then_0
          ;;[1 1 1] Decal and Effect
          (if (Variables|Default|GetDecalsOn)
            (Rendering|Decal|SpawnDecalatLocation (Variables|Default|GetFoot_R) (Math|Vector|MakeVector 1.0 _footprint_size _footprint_size) (Variables|Default|GetFootprint%20Location) _returnvalue_4 (Variables|Default|GetFootprint%20Lifetime))))
        (:then_1
          (if (Variables|Default|GetEffectOn)
            (Effects|SpawnEmitteratLocation "/Game/InfinityBladeEffects/Effects/FX_Combat_Base/Notifies/P_FootSteps_Walk.P_FootSteps_Walk" (Variables|Default|GetFootprint%20Location) _returnvalue_4)))
        (:then_2
          (goto _label))))))

(event EventBeginPlay
  (if (Variables|Default|GetStartInstant)
    (CallFunction|StartFootprint)))

(fn ConstructionScript)