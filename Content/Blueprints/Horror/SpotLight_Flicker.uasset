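; Horror spotlight actor that bursts into random flickering while lit, with buzz and flicker sounds.
; LightGoesOn, run at BeginPlay if LightInstantOn is set or callable later, shows the light, starts the buzz and enables flickering.
; Tick waits a random interval, then loops visibility toggles through a RetriggerableDelay up to a random count before restoring the light.
; PlaySound attaches sounds using an attenuation asset, otherwise adjusted attenuation with fade-in.
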(event Custom|LightGoesOn
  ;[1 1 1] Endless Buzz Sound + Switch Sound On
  (Utilities|FlowControl|Sequence
    (:then_0
      (Rendering|SetVisibility (Variables|Default|GetSpotLight) true false)
      ;;[1 1 1] Buzzsound
      (CallFunction|PlaySound (Variables|Default|GetBuzzSound) (Variables|Default|GetSpotLight) (Variables|Default|GetCustom%20Attenuation%20Setting) (Variables|Default|GetAttenuation%20Setting) 0.8 0.5))
    (:then_1
      (Variables|Default|SetLightInstantOn true))))

(event EventTick
  (params (DeltaSeconds :type Float%20%28single-precision%29))
  ;[1 1 1] Flicker Sound Roation
  (if (Variables|Default|GetLightInstantOn)
    (Utilities|FlowControl|Delay (Math|Random|RandomFloatinRange (Variables|Default|GetDelayLightONMin) (Variables|Default|GetDelayLightONMax)))
    (if (<= (Variables|Default|GetCurFlickerCount) (Math|Random|RandomFloatinRange (Variables|Default|GetFlickerCountMin) (Variables|Default|GetFlickerCountMax))) :!label _label
      (bind _result (Math|Float|IncrementFloat (Variables|Default|GetCurFlickerCount))
        (:%20%20
          (Variables|Default|SetCurFlickerCount _result)
          (Utilities|FlowControl|RetriggerableDelay (Math|Random|RandomFloatinRange (Variables|Default|GetDelayMin) (Variables|Default|GetDelayMax)))
          ;;[1 1 1] Flickersound
          (CallFunction|PlaySound (Variables|Default|GetFlickerSound) (Variables|Default|GetSpotLight) (Variables|Default|GetCustom%20Attenuation%20Setting) (Variables|Default|GetAttenuation%20Setting) 0.0 1.0)
          (Rendering|ToggleVisibility (Variables|Default|GetSpotLight) false)
          (goto _label)))
      (else
        (Variables|Default|SetCurFlickerCount 0.0)
        (Rendering|SetVisibility (Variables|Default|GetSpotLight) true false)))))

(event EventBeginPlay
  ;[1 1 1] Turn Light off when LightOn is inactive
  (if (Variables|Default|GetLightInstantOn)
    (CallFunction|LightGoeson)
    (else
      (Rendering|SetVisibility (Variables|Default|GetSpotLight) false false))))

(fn ConstructionScript)

(fn PlaySound
  (params (Sound :type Sound%20Wave%20Object%20Reference) (Attach :type Scene%20Component%20Object%20Reference) (Use%20Attenuation :type Attenuation%20Settings%20Structure) (Custom%20Attenuation :type Sound%20Attenuation%20Object%20Reference) (Fade%20Duration :type Float%20%28single-precision%29) (Fade%20Volume%20Level :type Float%20%28single-precision%29))
  (if (Utilities|IsValid Custom%20Attenuation)
    ;[1 1 1] Use Attenuation Settings
    (bind _returnvalue (Audio|SpawnSoundAttached Sound Attach "None" "0, 0, 0" "0, 0, 0" "KeepRelativeOffset" false 1.0 1.0 0.0 Custom%20Attenuation))
    (else
      ;[1 1 1] Use custom Attenuation
      (bind _returnvalue_2 (Audio|SpawnSoundAttached Sound Attach))
      (Utilities|FlowControl|Sequence
        (:then_1
          (Audio|Components|Audio|AdjustAttenuation _returnvalue_2 Use%20Attenuation))
        (:then_2
          (Audio|Components|Audio|FadeIn _returnvalue_2 Fade%20Duration Fade%20Volume%20Level 0.0 :!class /Script/Engine.AudioComponent))))))