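; Horror door actor that slams shut once, the first time anything overlaps its trigger box.
; A timeline lerps the door's yaw between configurable angles, using actor time dilation to scale the closing duration, then plays an attenuated slam sound at the door.
; The construction script applies the exposed trigger box transform and starting door angle.
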(event OnComponentBeginOverlap(Trigger)
  (params (OverlappedComponent :type Primitive%20Component%20Object%20Reference) (OtherActor :type Actor%20Object%20Reference) (OtherComp :type Primitive%20Component%20Object%20Reference) (OtherBodyIndex :type Integer) (bFromSweep :type Boolean) (SweepResult :type Hit%20Result%20Structure%20%28by%20ref%29))
  ;[1 1 1] Rotate Door
  (if (not (Variables|Default|GetIsClosed))
    (Variables|Default|SetIsClosed true)
    (bind _doorangle (Timeline|Timeline_Closedoor Play)
      (:Update
        (Variables|Default|SetCustomTimeDilation (/ 1.0 (Variables|Default|GetTime%20to%20Close)))
        (Transformation|SetRelativeRotation (Variables|Default|GetDoor_01) (Math|Rotator|MakeRotator 0.0 0.0 (Math|Float|Lerp (Variables|Default|GetDoor%20End) (Variables|Default|GetDoor%20Start) _doorangle)) false false))
      (:Finished
        ;[1 1 1] Play Sound
        (Audio|SpawnSoundAttached (Variables|Default|GetDoor%20Slam%20Sound) (Variables|Default|GetDoor_01) "None" (Transformation|GetWorldLocation (Variables|Default|GetDoor_01)) "0, 0, 0" "KeepRelativeOffset" false 1.0 1.0 0.0 (Variables|Default|GetSound%20Attenuation))))))

(fn ConstructionScript
  ;[1 1 1] Change the Overlapbox
  (Utilities|FlowControl|Sequence
    (:then_0
      (Transformation|SetRelativeTransform (Variables|Default|GetTrigger) (Math|Transform|MakeTransform (Variables|Default|GetOverlapBoxPosition) (Variables|Default|GetOverlapBoxRotation) (Variables|Default|GetOverlapBoxScale)) false false))
    (:then_1
      ;[1 1 1] Change the Door
      (Transformation|SetRelativeRotation (Variables|Default|GetDoor_01) (Math|Rotator|MakeRotator 0.0 0.0 (Variables|Default|GetDoor%20Start)) false false))))