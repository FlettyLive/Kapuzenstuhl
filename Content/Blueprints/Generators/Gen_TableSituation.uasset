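; Table situation generator that randomly dresses a scene with object packs when play begins.
; BeginPlay builds an array of ten pack classes, then spawns one random pick in each of four box components.
; Each spawn gets a random point from the box's scaled extent, ignoring box rotation, and a random yaw.
; The inclusive random index reaches the array length, so a pick can fall out of range.
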(event EventBeginPlay
  (bind _box1 (Variables|Default|GetBox1))
  (bind _box2 (Variables|Default|GetBox2))
  (bind _box3 (Variables|Default|GetBox3))
  (bind _box4 (Variables|Default|GetBox4))
  (bind _returnvalue (Components|Box|GetScaledBoxExtent _box1))
  (bind _returnvalue_2 (Components|Box|GetScaledBoxExtent _box2))
  (bind _returnvalue_3 (Components|Box|GetScaledBoxExtent _box3))
  (bind _returnvalue_4 (Components|Box|GetScaledBoxExtent _box4))
  (bind (_x _y _z) (Math|Vector|BreakVector _returnvalue))
  (bind (_x_2 _y_2 _z_2) (Math|Vector|BreakVector _returnvalue_2))
  (bind (_x_3 _y_3 _z_3) (Math|Vector|BreakVector _returnvalue_3))
  (bind (_x_4 _y_4 _z_4) (Math|Vector|BreakVector _returnvalue_4))
  ;[1 1 1] Array der Objekte erstellen
  (bind _output_get (Variables|Default|SetTableObjects (Utilities|Array|MakeArray "/Game/Blueprints/Generators/Packages/Pack_1.Pack_1_C" "/Game/Blueprints/Generators/Packages/Pack_2.Pack_2_C" "/Game/Blueprints/Generators/Packages/Pack_3.Pack_3_C" "/Game/Blueprints/Generators/Packages/Pack_4.Pack_4_C" "/Game/Blueprints/Generators/Packages/Pack_5.Pack_5_C" "/Game/Blueprints/Generators/Packages/Pack_6.Pack_6_C" "/Game/Blueprints/Generators/Packages/Pack_7.Pack_7_C" "/Game/Blueprints/Generators/Packages/Pack_8.Pack_8_C" "/Game/Blueprints/Generators/Packages/Pack_9.Pack_9_C" "/Game/Blueprints/Generators/Packages/Pack_10.Pack_10_C")))
  (Variables|Default|SetTableObjects_L (Utilities|Array|Length _output_get))
  (Utilities|FlowControl|Sequence
    (:then_0
      ;[1 1 1] Set Box1 Spawn
      (bind _output_get_2 (Variables|Default|SetBox1_Position (+ (Math|Vector|MakeVector (Math|Random|RandomFloatinRange (* _x -1.0) _x) (Math|Random|RandomFloatinRange (* _y -1.0) _y) (Math|Random|RandomFloatinRange (* _z -1.0) _z)) (Transformation|GetWorldLocation (Variables|Default|GetBox1)))))
      ;[1 1 1] Spawn und rotieren Pack 1
      (Game|SpawnActorfromClass (Utilities|Array|Get(acopy) (Variables|Default|GetTableObjects) (Math|Random|RandomIntegerinRange 0 (Variables|Default|GetTableObjects_L))) (Math|Transform|MakeTransform _output_get_2 (Math|Rotator|MakeRotator 0.0 0.0 (Math|Random|RandomFloatinRange 0.0 3.6e+02)) "1.000000,1,1") "Undefined" 0 0))
    (:then_1
      ;[1 1 1] Set Box2 Spawn
      (bind _output_get_3 (Variables|Default|SetBox2_Position (+ (Math|Vector|MakeVector (Math|Random|RandomFloatinRange (* _x_2 -1.0) _x_2) (Math|Random|RandomFloatinRange (* _y_2 -1.0) _y_2) (Math|Random|RandomFloatinRange (* _z_2 -1.0) _z_2)) (Transformation|GetWorldLocation (Variables|Default|GetBox2)))))
      ;[1 1 1] Spawn und rotieren Pack 1
      (Game|SpawnActorfromClass (Utilities|Array|Get(acopy) (Variables|Default|GetTableObjects) (Math|Random|RandomIntegerinRange 0 (Variables|Default|GetTableObjects_L))) (Math|Transform|MakeTransform _output_get_3 (Math|Rotator|MakeRotator 0.0 0.0 (Math|Random|RandomFloatinRange 0.0 3.6e+02)) "1.000000,1,1") "Undefined" 0 0))
    (:then_2
      ;[1 1 1] Set Box3 Spawn
      (bind _output_get_4 (Variables|Default|SetBox3_Position (+ (Math|Vector|MakeVector (Math|Random|RandomFloatinRange (* _x_3 -1.0) _x_3) (Math|Random|RandomFloatinRange (* _y_3 -1.0) _y_3) (Math|Random|RandomFloatinRange (* _z_3 -1.0) _z_3)) (Transformation|GetWorldLocation (Variables|Default|GetBox3)))))
      ;[1 1 1] Spawn und rotieren Pack 1
      (Game|SpawnActorfromClass (Utilities|Array|Get(acopy) (Variables|Default|GetTableObjects) (Math|Random|RandomIntegerinRange 0 (Variables|Default|GetTableObjects_L))) (Math|Transform|MakeTransform _output_get_4 (Math|Rotator|MakeRotator 0.0 0.0 (Math|Random|RandomFloatinRange 0.0 3.6e+02)) "1.000000,1,1") "Undefined" 0 0))
    (:then_3
      ;[1 1 1] Set Box4 Spawn
      (bind _output_get_5 (Variables|Default|SetBox4_Position (+ (Math|Vector|MakeVector (Math|Random|RandomFloatinRange (* _x_4 -1.0) _x_4) (Math|Random|RandomFloatinRange (* _y_4 -1.0) _y_4) (Math|Random|RandomFloatinRange (* _z_4 -1.0) _z_4)) (Transformation|GetWorldLocation (Variables|Default|GetBox4)))))
      ;[1 1 1] Spawn und rotieren Pack 1
      (Game|SpawnActorfromClass (Utilities|Array|Get(acopy) (Variables|Default|GetTableObjects) (Math|Random|RandomIntegerinRange 0 (Variables|Default|GetTableObjects_L))) (Math|Transform|MakeTransform _output_get_5 (Math|Rotator|MakeRotator 0.0 0.0 (Math|Random|RandomFloatinRange 0.0 3.6e+02)) "1.000000,1,1") "Undefined" 0 0))))

(fn ConstructionScript)