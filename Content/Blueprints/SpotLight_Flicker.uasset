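; Flickering spotlight Blueprint that starts dark or lit based on LightOn, with bulb buzz and switch sounds.
; LightGoesOn shows the light, fades in the buzz, plays the switch sound and sets LightOn.
; While on, Tick uses a random Delay between bursts, then loops through RetriggerableDelay, toggling visibility with a flicker sound.
; The burst limit is re-randomized on each pass; when exceeded, the count resets and the light stays visible.
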(event Custom|LightGoesOn
  (bind _bulb_buzz (Variables|Default|Getbulb_buzz))
  ;[1 1 1] Endless Buzz Sound + Switch Sound On
  (Utilities|FlowControl|Sequence
    (:then_0
      (Rendering|SetVisibility (Variables|Default|GetSpotLight) true false)
      (Components|Activation|Activate (Variables|Default|Getbulb_buzz) true)
      (Audio|Components|Audio|FadeIn _bulb_buzz 0.8 0.5 0.0 :!class /Script/Engine.AudioComponent)
      (Audio|SpawnSoundAttached "/Game/SoundCues/Light_Switch_On.Light_Switch_On" _bulb_buzz))
    (:then_1
      (Variables|Default|SetLightOn true))))

(event EventTick
  (params (DeltaSeconds :type Float%20%28single-precision%29))
  ;[1 1 1] Flicker Sound Roation
  (if (Variables|Default|GetLightOn)
    (Utilities|FlowControl|Delay (Math|Random|RandomFloatinRange (Variables|Default|GetDelayLightONMin) (Variables|Default|GetDelayLightONMax)))
    (if (<= (Variables|Default|GetCurFlickerCount) (Math|Random|RandomFloatinRange (Variables|Default|GetFlickerCountMin) (Variables|Default|GetFlickerCountMax))) :!label _label
      (bind _result (Math|Float|IncrementFloat (Variables|Default|GetCurFlickerCount))
        (:%20%20
          (Variables|Default|SetCurFlickerCount _result)
          (Utilities|FlowControl|RetriggerableDelay (Math|Random|RandomFloatinRange (Variables|Default|GetDelayMin) (Variables|Default|GetDelayMax)))
          (Audio|SpawnSoundAttached "/Game/SoundCues/Bulb_Flicker.Bulb_Flicker" (Variables|Default|GetSpotLight) "None" "0, 0, 0" "0, 0, 0" "KeepRelativeOffset" false 1.0)
          (Rendering|ToggleVisibility (Variables|Default|GetSpotLight) false)
          (goto _label)))
      (else
        (Variables|Default|SetCurFlickerCount 0.0)
        (Rendering|SetVisibility (Variables|Default|GetSpotLight) true false)))))

(event EventBeginPlay
  ;[1 1 1] Turn Light off when LightOn is inactive
  (if (Variables|Default|GetLightOn)
    (CallFunction|LightGoeson)
    (else
      (Rendering|SetVisibility (Variables|Default|GetSpotLight) false false))))

(fn ConstructionScript)