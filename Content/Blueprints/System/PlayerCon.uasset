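; Player controller that handles camera look with view limits, pause menu toggling and forwarding of the action press to the pawn.
; The D key starts a head-shake test that samples mouse X every 0.1 seconds and prints "No" for enough large leftward jumps, otherwise "Yes".
; While paused, Tick times vertical mouse stillness and plays a one-off door-slam jumpscare when movement resumes after a random threshold.
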(event Custom|StartYesNo
  (bind _mousex_array (Variables|Default|GetMouseX_Array))
  ;[1 1 1] Yes No Function
  ;;[1 1 1] Reset Values
  (Utilities|Array|Clear (Variables|Default|GetMouseX_Array))
  (Variables|Default|SetYesNoTimerCount 0)
  (Variables|Default|SetYesNoWorked_X 0)
  ;;[1 1 1] Add the Mouse X Value to the Array
  (Utilities|FlowControl|Delay 0.1 :!label _label)
  (bind _x (Class|LowEntryExtendedStandardLibrary|GetMousePosition))
  (bind _output_get (Variables|Default|SetMouseX (Math|Conversions|ToFloat(Integer) _x)))
  (Utilities|Array|Add (Variables|Default|GetMouseX_Array) _output_get)
  (Variables|Default|SetYesNoTimerCount (+ (Variables|Default|GetYesNoTimerCount) 1))
  (if (<= (Variables|Default|GetYesNoTimerCount) 10)
    (goto _label)
    (else
      (Variables|Default|SetYesNoTimerCount 0)
      (Development|PrintString "" false false "(R=0.000000,G=0.660000,B=1.000000,A=1.000000)" 0.0 :!label _label_2)
      (if (or (< (- (Utilities|Array|Get(acopy) _mousex_array (+ (Variables|Default|GetYesNoTimerCount) 1)) (Utilities|Array|Get(acopy) _mousex_array (Variables|Default|GetYesNoTimerCount))) -16.0) (> (- (Utilities|Array|Get(acopy) _mousex_array (Variables|Default|GetYesNoTimerCount)) (Utilities|Array|Get(acopy) _mousex_array (+ (Variables|Default|GetYesNoTimerCount) 1))) 16.0))
        ;;[1 1 1] Only raise the OK X Value if higher than 16
        (Variables|Default|SetYesNoWorked_X (+ (Variables|Default|GetYesNoWorked_X) 1)))
      (Variables|Default|SetYesNoTimerCount (+ (Variables|Default|GetYesNoTimerCount) 1))
      (if (<= (Variables|Default|GetYesNoTimerCount) 10)
        (goto _label_2)
        (elif (> (Variables|Default|GetYesNoWorked_X) 3)
          (Development|PrintString "No")
          (else
            (Development|PrintString "Yes")))))))

(event EventBeginPlay
  (bind _returnvalue (Game|GetPlayerCameraManager 0))
  ;[1 1 1] Cameralock
  (Utilities|FlowControl|Sequence
    (:then_0
      (Variables|/Script/Engine.PlayerCameraManager|SetViewPitchMin _returnvalue -65.0))
    (:then_1
      (Variables|/Script/Engine.PlayerCameraManager|SetViewPitchMax _returnvalue 45.0))
    (:then_2
      (Variables|/Script/Engine.PlayerCameraManager|SetViewYawMin _returnvalue 1.9e+02))
    (:then_3
      (Variables|/Script/Engine.PlayerCameraManager|SetViewYawMax _returnvalue -1e+01))
    (:then_4
      ;[1 1 1] PauseJumpScare Settings
      (Variables|Default|SetPauseTimerJumpScare (Math|Random|RandomFloatinRange 5.0 1e+01)))))

(event EventTick
  (params (DeltaSeconds :type Float%20%28single-precision%29))
  (Utilities|FlowControl|Sequence
    (:then_1
      ;[1 1 1] JumpScare for Pausescreen Preperation
      (if (Game|IsGamePaused)
        (if (not (Variables|Default|GetPauseJumpScare))
          (bind _y (Class|LowEntryExtendedStandardLibrary|GetMousePosition))
          (Variables|Default|SetMouseX 0.0)
          (Variables|Default|SetMouseY _y)
          (if (Math|Boolean|Equal(Boolean) (== 0 (Variables|Default|GetMouseX_Prev)) (== (Variables|Default|GetMouseY_Prev) (Variables|Default|GetMouseY)))
            (Variables|Default|SetTimer (+ (Variables|Default|GetTimer) 0.01))
            (Variables|Default|SetMouseX_Prev 0 :!label _label)
            (Variables|Default|SetMouseY_Prev (Variables|Default|GetMouseY))
            (elif (>= (Variables|Default|GetTimer) (Variables|Default|GetPauseTimerJumpScare))
              (Variables|Default|SetTimer 0.0)
              (Audio|PlaySound2D "/Game/Sounds/doorslam_1.doorslam_1")
              (Variables|Default|SetPauseJumpScare true)
              (goto _label))))))))

(event Input|ActionEvents|InputActionFireTrace
  (params (Key :type Key%20Structure :default "AnyKey"))
  ;[1 1 1] Cam Movement
  (:Pressed
    (Class|PlayerBPI|ActionButtonF(Message) (Pawn|GetControlledPawn))))

(event Input|AxisEvents|InputAxisLookUp
  (params (AxisValue :type Float%20%28single-precision%29))
  ;[1 1 1] Cam Movement
  (Class|PlayerController|AddPitchInput AxisValue))

(event Input|AxisEvents|InputAxisTurn
  (params (AxisValue :type Float%20%28single-precision%29))
  ;[1 1 1] Cam Movement
  (Class|PlayerController|AddYawInput AxisValue))

(event Input|KeyboardEvents|P
  (params (Key :type Key%20Structure :default "AnyKey"))
  ;[1 1 1] Call Pause
  (:Pressed
    (bind _asgame_hud (Utilities|Casting|CastToGameHUD (HUD|GetHUD)))
    (if (Game|IsGamePaused)
      (Default|HidePauseMenu _asgame_hud)
      (else
        (Default|ShowPauseMenu _asgame_hud)
        ;[1 1 1] PauseJumpScare Settings
        (Variables|Default|SetPauseJumpScare false)))))

(event Input|KeyboardEvents|D
  (params (Key :type Key%20Structure :default "AnyKey"))
  ;[1 1 1] Yes No Function
  (:Released
    (Variables|Default|SetYesNoTimerCount 0)
    (CallFunction|StartYesNo)))

(fn ConstructionScript)

(fn GetYesNo
  (params (MouseX :type Integer) (MouseY :type Integer)))