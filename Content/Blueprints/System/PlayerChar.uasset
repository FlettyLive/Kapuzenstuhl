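; Player character that shows a crosshair and lets the player hit objects in view with a trace.
; On BeginPlay, CreateHUD creates the Crossair widget and adds it to the viewport.
; The ActionButtonF event runs a short-range Visibility line trace forward from PlayerCamera.
; Hit actors that implement the TartetBPI interface receive HandleWasHitMessage, so each target decides its own response.
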(event EventBeginPlay
  ;[1 1 1] Create HUD Interface
  (CallFunction|CreateHUD))

(event EventActionButtonF
  (bind _playercamera (Variables|Default|GetPlayerCamera))
  (bind _returnvalue (Transformation|GetWorldLocation _playercamera))
  ;[1 1 1] Fire Trace
  (bind (_outhit _returnvalue_2) (Collision|LineTraceByChannel _returnvalue (+ _returnvalue (* (Math|Vector|GetForwardVector (Transformation|GetWorldRotation _playercamera)) 1e+03)) "TraceTypeQuery1" false 0 "None"))
  (if _returnvalue_2
    (if (Utilities|DoesObjectImplementInterface (.HitActor (Collision|BreakHitResult _outhit)) "/Game/Blueprints/Targets/TartetBPI.TartetBPI_C")
      (Class|TartetBPI|HandleWasHit(Message) (.HitActor (Collision|BreakHitResult _outhit))))))

(fn ConstructionScript)

(fn CreateHUD
  (bind _returnvalue (UserInterface|CreateWidget "/Game/Blueprints/UI/Crossair.Crossair_C"))
  (UserInterface|Viewport|AddtoViewport _returnvalue 0))