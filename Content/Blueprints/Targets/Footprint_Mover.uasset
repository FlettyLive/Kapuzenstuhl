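; Footprint_Mover is an invisible actor that travels along a trail of footprints and triggers each one as it passes.
; HandleWasHit stores the current location, then plays a timeline whose vector output is added to that start point to move the actor without sweeping.
; On each overlap, it takes the first overlapping Footprint_L and Footprint_R and calls PlayFootstep on them.
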(event EventHandleWasHit
  ;[1 1 1] Bewege den unsichtbaren Mover entlang der Fußspuren
  (Variables|Default|SetFootstepMover (Transformation|GetActorLocation))
  (bind _footstepmover (Timeline|FootstepMover_Timerline PlayFromStart)
    (:Update
      (Transformation|SetActorLocation (+ _footstepmover (Variables|Default|GetFootstepMover)) false false))))

(event Collision|EventActorBeginOverlap
  (params (OtherActor :type Actor%20Object%20Reference))
  ;[1 1 1] Wenn Fußspur überlappt, spiele diese ab
  (Utilities|FlowControl|Sequence
    (:then_0
      (bind _asfootprint_l (Utilities|Casting|CastToFootprint_L (Utilities|Array|Get(acopy) (Collision|GetOverlappingActors "/Game/Blueprints/Footprint_L.Footprint_L_C" :!class /Script/Engine.Actor))))
      (Default|PlayFootstep _asfootprint_l))
    (:then_1
      (bind _asfootprint_r (Utilities|Casting|CastToFootprint_R (Utilities|Array|Get(acopy) (Collision|GetOverlappingActors "/Game/Blueprints/Footprint_R.Footprint_R_C" :!class /Script/Engine.Actor))))
      (Default|PlayFootstep _asfootprint_r))))

(fn ConstructionScript)