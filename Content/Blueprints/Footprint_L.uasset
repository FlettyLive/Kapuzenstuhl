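; Left footprint actor that stays out of sight at runtime until it is triggered to appear on the ground with a footstep sound.
; BeginPlay moves it to a fixed height in the air, so it is hidden in game while remaining visible in the editor.
; PlayFootstep captures the current location, runs a timeline whose movement offset brings the print to the floor, and plays the sound at that captured location.
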(event Custom|PlayFootstep
  ;[1 1 1] Fußspur auf Boden bewegen
  (Variables|Default|SetInitial%20Location (Transformation|GetActorLocation))
  (Utilities|FlowControl|Sequence
    (:then_0
      (bind _movement (Timeline|Footprint_Timeline PlayFromStart)
        (:Update
          (Transformation|SetActorLocation (+ _movement (Variables|Default|GetInitial%20Location)) false false))))
    (:then_1
      (Audio|PlaySoundatLocation "/Game/SoundCues/Footsteps_1.Footsteps_1" (Variables|Default|GetInitial%20Location)))))

(event EventBeginPlay
  (bind _returnvalue (Transformation|GetActorLocation))
  (bind (_x _y) (Math|Vector|BreakVector _returnvalue))
  ;[1 1 1] Abdruck in die Luft setzten damit nicht direkt sichtbar (aber im Editor)
  (Variables|Default|SetInitial%20Location _returnvalue)
  (Transformation|SetActorLocation (Math|Vector|MakeVector _x _y 4e+01) false false))

(fn ConstructionScript)